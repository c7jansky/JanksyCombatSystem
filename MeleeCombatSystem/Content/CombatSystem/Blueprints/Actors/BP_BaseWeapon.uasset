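; Base weapon actor that attaches to its owner, supplies attack, dodge and combat-toggle montages by action type, and deals damage on hit.
; On equip it attaches to the hand or holster socket by combat state, registers with the owner's combat component and updates the AnimInstance combat type.
; Its collision component, ignoring the owner, reports hits, applying point damage to receptive actors.
; It can also switch its mesh to simulated physics.
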(event `self.BP_CollisionComponent.OnHit`
  (params (HitResult :type "HitResult Structure"))
  (bind (_bblockinghit _binitialoverlap _time _distance _location _impactpoint _normal _impactnormal _physmat _hitactor) (`GameplayStatics.BreakHitResult` HitResult))
  (bind _returnvalue (message `/Game/CombatSystem/Blueprints/Interfaces/CombatBPI.CanRecieveDamage` _hitactor))
  (if _returnvalue
    (`GameplayStatics.ApplyPointDamage` _hitactor (`self.Damage`) (`self.GetActorForwardVector` (`self.GetOwner`)) HitResult (`self.GetInstigatorController`) self)))

(event `SimulateWeaponPhysics`
  (bind _return_value (`self.GetItemMesh`))
  (`PrimitiveComponent.SetCollisionProfileName` _return_value "PhysicsActor" true)
  (`PrimitiveComponent.SetSimulatePhysics` _return_value true))

(fn `GetActionMontages`
  (params (Index :type "/Game/CombatSystem/Blueprints/Enums/E_CharacterAction Enum" :default "NewEnumerator0"))
  (returns (Montages :type "Array of AnimMontage Object Reference"))
  (return (select `/Game/CombatSystem/Blueprints/Enums/E_CharacterAction` Index :`NewEnumerator1` (`self.LightAttackMontages`) :`NewEnumerator2` (`self.HeavyAttackMontages`) :`NewEnumerator3` (`self.ChargedAttackMontages`) :`NewEnumerator4` (`self.FallingAttackMontages`) :`NewEnumerator9` (`self.Sprint Attack Montages`) :`NewEnumerator5` (`self.DodgeMontages`) :`NewEnumerator6` (`|MakeArray` (`self.EnterCombat`)) :`NewEnumerator7` (`|MakeArray` (`self.ExitCombat`)))))

(fn `OnEquipped`
  (`self.SetIsEquipped` true)
  (set `self.CombatCombatComponent` (`self.GetComponentByClass` (`self.GetOwner`) "/Game/CombatSystem/Blueprints/Components/BP_CombatComponent.BP_CombatComponent_C"))
  (`self.AttachActor` (select `bool` (`/Game/CombatSystem/Blueprints/Components/BP_CombatComponent.IsCombatEnabled?` (`self.CombatCombatComponent`)) :`false` (`self.Attach Socket Name`) :`true` (`self.HandSocketName`)))
  (`/Game/CombatSystem/Blueprints/Components/BP_CombatComponent.SetMainWeapon` (`self.CombatCombatComponent`) self)
  (message `/Game/CombatSystem/Blueprints/Interfaces/AnimInstanceBPI.UpdateCombatType` (`SkeletalMeshComponent.GetAnimInstance` (`Character.Mesh` (cast `Character` (`self.GetOwner`) :!pure true))) (`self.CombatType`))
  (`/Game/CombatSystem/Blueprints/Components/BP_CollisionComponent.SetCollisionMesh` (`self.BP_CollisionComponent`) (`self.GetItemMesh`))
  (`/Game/CombatSystem/Blueprints/Components/BP_CollisionComponent.AddActorToIgnore` (`self.BP_CollisionComponent`) (`self.GetOwner`)))

(fn `UserConstructionScript`
  (`parent.UserConstructionScript`))